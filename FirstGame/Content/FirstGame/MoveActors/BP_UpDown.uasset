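; BP_UpDown is an actor whose static mesh bobs continuously up and down along the vertical axis.
; Each Tick steps a stored Z value by a fixed amount and applies it as the mesh's relative location.
; A boolean flips direction at the upper and lower height limits, and the speed depends on frame rate because delta time is not used.
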(event `self.ReceiveTick`
  (params (DeltaSeconds :type "Float (single-precision)"))
  (if (`self.IsMoveUp`)
    (bind _output_get (set `self.LocZ` (+ (`self.LocZ`) 10.0)))
    (`SceneComponent.K2_SetRelativeLocation` (`self.StaticMesh`) (`KismetMathLibrary.MakeVector` 0.0 0.0 _output_get) false false)
    (if (>= (`self.LocZ`) 500.0)
      (set `self.IsMoveUp` false))
    (else
      (bind _output_get_2 (set `self.LocZ` (- (`self.LocZ`) 10.0)))
      (`SceneComponent.K2_SetRelativeLocation` (`self.StaticMesh`) (`KismetMathLibrary.MakeVector` 0.0 0.0 _output_get_2) false false)
      (if (<= (`self.LocZ`) 0.0)
        (set `self.IsMoveUp` true)))))

(fn `UserConstructionScript`)